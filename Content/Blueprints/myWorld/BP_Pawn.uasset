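; First-person player pawn for grocery item interaction, with movement and mouse look that pause while HeldItem is valid.
; BeginPlay starts music, enables the trace interactor component and creates WBP_UI, whose crosshair fades through a timeline.
; Mouse clicks forward to the interactor, though right-button release also calls RightClickPress.
; AddingToList tallies item names in a map and rebuilds the UI list, while trace interface functions are stubs.
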(event Custom|DisableCrosshair
  ;[1 1 1] Init UI
  ;;[1 1 1] Init UI
  (bind _opacity (Timeline|Crosshair_Opacity Reverse)
    (:Update
      (Widget|SetRenderOpacity (stale EventBeginPlay _output_get) _opacity))))

(event Custom|EnableCrosshair
  ;[1 1 1] Init UI
  ;;[1 1 1] Init UI
  (bind _opacity (Timeline|Crosshair_Opacity Play)
    (:Update
      (Widget|SetRenderOpacity (stale EventBeginPlay _output_get) _opacity))))

(event EventBeginPlay
  ;[1 1 1] Beginplay- Turn on BPC Trace
  (Audio|PlaySound2D "/Game/Audio/ES_The_Cutest_Thing_-_Water_Mirrors.ES_The_Cutest_Thing_-_Water_Mirrors" 1.0 1.0 0.0 0 0)
  (Default|Enable (Variables|Default|GetBPC_TraceInteractor))
  ;[1 1 1] Init UI
  (bind _returnvalue (UserInterface|CreateWidget "/Game/Blueprints/myWorld/WBP_UI.WBP_UI_C"))
  (bind _output_get (Variables|Default|SetUI _returnvalue))
  ;;[1 1 1] Init UI
  (UserInterface|Viewport|AddtoViewport _returnvalue 0)
  (bind _opacity (Timeline|Crosshair_Opacity PlayFromStart)
    (:Update
      (Widget|SetRenderOpacity _output_get _opacity))))

(event Input|AxisEvents|InputAxisTurn
  (params (AxisValue :type Float%20%28single-precision%29))
  ;[1 1 1] InputAxis
  (Utilities|IsValid (Variables|Default|GetHeldItem)
    (:Is%20Not%20Valid
      (Pawn|Input|AddControllerYawInput (* AxisValue (Variables|Default|GetMouseSpeed))))))

(event Input|AxisEvents|InputAxisLookUp
  (params (AxisValue :type Float%20%28single-precision%29))
  ;[1 1 1] InputAxis
  (Utilities|IsValid (Variables|Default|GetHeldItem)
    (:Is%20Not%20Valid
      (Pawn|Input|AddControllerPitchInput (* AxisValue (Variables|Default|GetMouseSpeed))))))

(event Input|AxisEvents|InputAxisMoveRight
  (params (AxisValue :type Float%20%28single-precision%29))
  ;[1 1 1] InputAxis
  (Utilities|IsValid (Variables|Default|GetHeldItem)
    (:Is%20Not%20Valid
      (Pawn|Input|AddMovementInput (Transformation|GetActorRightVector) AxisValue false))))

(event Input|AxisEvents|InputAxisMoveForward
  (params (AxisValue :type Float%20%28single-precision%29))
  ;[1 1 1] InputAxis
  (Utilities|IsValid (Variables|Default|GetHeldItem) ; Check if Held item is Set, if not use movement input.
    (:Is%20Not%20Valid
      (Pawn|Input|AddMovementInput (Transformation|GetActorForwardVector) AxisValue false))))

(event Input|MouseEvents|LeftMouseButton
  (params (Key :type Key%20Structure :default "None"))
  (bind _self self)
  (bind _bpc_traceinteractor (Variables|Default|GetBPC_TraceInteractor))
  ;[1 1 1] Mouse Buttons + Trace Interaction
  (:Pressed
    (Default|LeftClickPress _bpc_traceinteractor _self) ; Cast to BP_GroceryItem via BPI
  )
  (:Released
    (Default|LeftClickRelease _bpc_traceinteractor _self)))

(event Input|MouseEvents|RightMouseButton
  (params (Key :type Key%20Structure :default "None"))
  ;[1 1 1] Mouse Buttons + Trace Interaction
  (:Pressed
    (Default|RightClickPress (Variables|Default|GetBPC_TraceInteractor) self :!label _label) ; Cast to BP_GroceryItem via BPI
  )
  (:Released
    (goto _label)))

(fn ConstructionScript)

(fn TraceActivateUp
  (params (Hit :type Hit%20Result%20Structure) (Instigator :type Pawn%20Object%20Reference))
  (return false))

(fn TraceActivateDown
  (params (Hit :type Hit%20Result%20Structure) (Instigator :type Pawn%20Object%20Reference))
  (return false))

(fn TraceMove
  (params (Hit :type Hit%20Result%20Structure%20%28by%20ref%29))
  (return false))

(fn TraceLeaveComponent
  (params (Hit :type Hit%20Result%20Structure) (Component :type Primitive%20Component%20Object%20Reference))
  (return false))

(fn TraceHitComponent
  (params (Hit :type Hit%20Result%20Structure) (Component :type Primitive%20Component%20Object%20Reference))
  (return false))

(fn TraceLeaveObject
  (params (Hit :type Hit%20Result%20Structure))
  (return false))

(fn TraceHitObject
  (params (Hit :type Hit%20Result%20Structure))
  (return false))

(fn AddStructtoList
  (params (newData :type S%20Data%20Structure))
  (Utilities|Array|Add (Variables|Default|GetdataArray) newData)
  (Default|AddDatatoList (Variables|Default|GetUI) newData))

(fn AddingtoList
  (params (itemName :type String))
  (bind _myhash (Variables|Default|GetmyHash))
  (bind _myhash_2 (Variables|Default|GetmyHash))
  (bind _output_get (Variables|Default|SetitemName itemName))
  (if (Utilities|Map|Contains _myhash _output_get)
    (CallFunction|UpDateHash)
    (else
      (Utilities|Map|Add _myhash _output_get 1)))
  (Class|ListView|ClearListItems (Variables|/Game/Blueprints/myWorld/WBP_UI.WBP_UI_C|GetmyListView (Variables|Default|GetUI)))
  (bind _keys (Utilities|Map|Keys _myhash_2))
  (bind _output_get_2 (Variables|Default|SetstringArraysKey _keys))
  (bind _values (Utilities|Map|Values _myhash_2))
  (for (_array_element _array_index) _output_get_2
    (CallFunction|AddStructtoList (Utilities|Struct|MakeSData _array_element (Utilities|Array|Get(acopy) _values _array_index)))))

(fn UpDateHash
  (bind _myhash (Variables|Default|GetmyHash))
  (bind _itemname (Variables|Default|GetitemName))
  (bind _keys (Utilities|Map|Keys (Variables|Default|GetmyHash)))
  (for (_array_element _array_index) _keys
    (if (Utilities|Enum|Equal(Enum) _array_element (Variables|Default|GetitemName))
      (bind _values (Utilities|Map|Values (Variables|Default|GetmyHash)))
      (bind _output_get (Variables|Default|SettempValue (Utilities|Array|Get(acopy) _values _array_index)))
      (bind _output_get_2 (Variables|Default|SettempValue (+ _output_get 1)))
      (Utilities|Map|Remove _myhash _itemname)
      (Utilities|Map|Add _myhash _itemname _output_get_2))))