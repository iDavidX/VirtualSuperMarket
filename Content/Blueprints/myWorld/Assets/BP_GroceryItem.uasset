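; BP_GroceryItem is an interactable grocery item that the player collects with a double click or holds to pick up and inspect.
; Pawn trace events toggle custom-depth highlighting and route clicks, with a MultiGate and short delay separating double click from hold.
; Collecting adds its name to the pawn's list, flashes materials, fades and destroys it.
; Holding fills UI progress, then lerps it before the trace interactor; right click toggles mouse rotation, and release reverses the lerp.
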(event Custom|DropItem
  (bind _pawn (Variables|Default|GetPawn))
  ;[1 1 1] Pick Up & Drop Item
  ;;[1 1 1] Drop Event
  (Variables|Default|SetIsPressed false)
  (if (not (Variables|Default|GetIsPickedUp))
    (CallFunction|StopHoldClick)
    (else
      ;;[1 1 1] Hold Click Functionality
      ;;;[0.1094 0.1094 0.1094] Detach from Pawn
      (Transformation|DetachFromComponent (Variables|Default|GetStaticMesh) "KeepWorld" "KeepWorld" "KeepWorld" true)
      (Rendering|SetRenderCustomDepth (Variables|Default|GetStaticMesh) true)
      ;;;[0.1094 0.1094 0.1094] Boolean Set
      (Variables|Default|SetIsPickedUp false)
      (Variables|/Game/Blueprints/myWorld/BP_Pawn.BP_Pawn_C|SetHeldItem (Variables|Default|GetPawn) 0)
      (Input|DisableInput (Game|GetPlayerController 0))
      (Default|EnableCrosshair (Variables|Default|GetPawn))
      (CallFunction|ResetMultiGate)
      ;;;[0.1094 0.1094 0.1094] Transform Actor Location
      (bind _alpha (Timeline|PickupTimeline Reverse)
        (:Update
          (if (> (.SphereRadius (Collision|GetComponentBounds (Variables|Default|GetStaticMesh))) 3e+01)
            (Variables|Default|SetEnd%20Loc (Utilities|TraceTransform _pawn 8e+01))
            (else
              (Variables|Default|SetEnd%20Loc (Utilities|TraceTransform _pawn 4e+01))))
          (Transformation|SetActorTransform (Math|Transform|Lerp(Transform) (Variables|Default|GetStart%20Loc) (Variables|Default|GetEnd%20Loc) _alpha)))))))

(event Custom|ResetMultiGate
  ;[1 1 1] RotateItem
  ;;[1 1 1] Activate input
  (Utilities|FlowControl|MultiGate false true -1) ; enters at Reset
)

(event Custom|RotateItem
  ;[1 1 1] RotateItem
  ;;[1 1 1] Activate input
  (Rendering|SetRenderCustomDepth (Variables|Default|GetStaticMesh) false)
  (Variables|/Game/Blueprints/myWorld/BP_Pawn.BP_Pawn_C|GetHeldItem (Variables|Default|GetPawn)
    (:then
      (Utilities|FlowControl|MultiGate false true -1
        (:Out%200
          (bind _output_get (Variables|Default|SetIsRotating true)))
        (:Out%201
          (Variables|Default|SetIsRotating false)))
      (Input|EnableInput (Game|GetPlayerController 0))
      (if (not _output_get)
        (Input|DisableInput 0)
        (Variables|Default|SetIsRotating false)))
    (:else
      (Input|DisableInput (Game|GetPlayerController 0))
      (Variables|Default|SetIsRotating false))))

(event Custom|PickupItem
  (bind _pawn (Variables|Default|GetPawn))
  (bind _pawn_2 (Variables|Default|GetPawn))
  (bind _bpc_traceinteractor (Variables|/Game/Blueprints/myWorld/BP_Pawn.BP_Pawn_C|GetBPC_TraceInteractor _pawn))
  ;[1 1 1] Pick Up & Drop Item
  ;;[1 1 1] Pickup Event
  (Variables|Default|SetIsPressed true)
  (if (not (Variables|Default|GetIsPickedUp))
    ;;[1 1 1] Double Click Functionality
    (Utilities|FlowControl|Sequence
      (:then_0
        (Utilities|FlowControl|MultiGate false false -1 :!label _label
          (:Out%201
            ;;;[0.1094 0.1094 0.1094] Activate Input
            (Utilities|FlowControl|DoOnce false
              (:Completed
                (CallFunction|StopHoldClick)
                (Variables|Default|SetIsCollected true)
                (Audio|PlaySound2D "/Game/Audio/ES_Chime_Bell_Muted_3_-_SFX_Producer.ES_Chime_Bell_Muted_3_-_SFX_Producer" 1.0 1.0 0.0 0 0)
                (Default|AddingtoList (Variables|Default|GetPawn) (Variables|Default|GetmyName))
                ;;;;[0.1094 0.1094 0.1094] Copy Original Materials for StaticMesh
                (Rendering|Material|SetCustomPrimitiveDataFloat (Variables|Default|GetStaticMesh) 0 1.0)
                (for _index (range 0 (- (Rendering|Material|GetNumMaterials (Variables|Default|GetStaticMesh)) 1))
                  (Utilities|Array|Add (Variables|Default|GetSM%20Material) (Rendering|Material|GetMaterial (Variables|Default|GetStaticMesh) _index)))
                (Utilities|ForLoopwithDelay 0 2 0.2
                  (:Loop%20Body
                    ;;;[0.1094 0.1094 0.1094] Flash Animation
                    (Utilities|FlowControl|FlipFlop
                      (:A
                        (for _index_2 (range 0 (- (Rendering|Material|GetNumMaterials (Variables|Default|GetStaticMesh)) 1))
                          (Rendering|Material|SetMaterial (Variables|Default|GetStaticMesh) _index_2 "/Game/Materials/M_FlashMaterial.M_FlashMaterial")))
                      (:B
                        (for _index_3 (range 0 (- (Rendering|Material|GetNumMaterials (Variables|Default|GetStaticMesh)) 1))
                          (Rendering|Material|SetMaterial (Variables|Default|GetStaticMesh) _index_3 (Utilities|Array|Get(acopy) (Variables|Default|GetSM%20Material) _index_3))))))
                  (:Completed
                    ;;;[0.1094 0.1094 0.1094] Disappear Animation & DestroyActor
                    (bind _opacity (Timeline|Collected%20Opacity PlayFromStart)
                      (:Update
                        (Rendering|Material|SetCustomPrimitiveDataFloat (Variables|Default|GetStaticMesh) 0 _opacity))
                      (:Finished
                        (Actor|DestroyActor))))))))))
      (:then_1
        (Utilities|FlowControl|Delay 0.3) ; Hold Click Time
        (if (and (Variables|Default|GetIsPressed) (not (Variables|Default|GetIsCollected)))
          (Utilities|FlowControl|Sequence ; If not double clicked within certain delay, will switch to hold click functionality
            (:then_0
              (goto _label Reset))
            (:then_1
              ;;[1 1 1] Hold Click Functionality
              ;;;[0.1094 0.1094 0.1094] Activate Input
              (bind _progression (Timeline|HoldItem_Progress PlayFromStart)
                (:Update
                  (Default|ProgressAlpha (Variables|/Game/Blueprints/myWorld/BP_Pawn.BP_Pawn_C|GetUI (Variables|Default|GetPawn)) _progression))
                (:Finished
                  (CallFunction|StopHoldClick)
                  ;;;[0.1094 0.1094 0.1094] Attach to Pawn
                  (Rendering|SetRenderCustomDepth (Variables|Default|GetStaticMesh) false)
                  (Variables|Default|SetEnd%20Loc (Math|Transform|MakeTransform (+ (Transformation|GetWorldLocation _bpc_traceinteractor) (* (Math|Vector|GetForwardVector _bpc_traceinteractor) 6e+01)) (.rotation (Variables|Default|GetStart%20Loc)) (.scale (Transformation|GetWorldTransform _bpc_traceinteractor))))
                  (Transformation|SetMobility (Variables|Default|GetStaticMesh) "Movable")
                  (Transformation|AttachComponentToComponent (Variables|/Game/Blueprints/myWorld/BP_Pawn.BP_Pawn_C|GetBPC_TraceInteractor (Variables|Default|GetPawn)) "None" "KeepWorld" "KeepWorld" "KeepWorld" true)
                  ;;;[0.1094 0.1094 0.1094] Boolean Set
                  (Variables|Default|SetIsPickedUp true)
                  (Variables|/Game/Blueprints/myWorld/BP_Pawn.BP_Pawn_C|SetHeldItem (Variables|Default|GetPawn) self)
                  (Default|DisableCrosshair (Variables|Default|GetPawn))
                  (Utilities|FlowControl|Sequence
                    (:then_0
                      ;;;[0.1094 0.1094 0.1094] Transform Actor Location
                      (bind _alpha (Timeline|PickupTimeline Play)
                        (:Update
                          (if (> (.SphereRadius (Collision|GetComponentBounds (Variables|Default|GetStaticMesh))) 3e+01)
                            (Variables|Default|SetEnd%20Loc (Utilities|TraceTransform _pawn_2 8e+01))
                            (else
                              (Variables|Default|SetEnd%20Loc (Utilities|TraceTransform _pawn_2 4e+01))))
                          (Transformation|SetActorTransform (Math|Transform|Lerp(Transform) (Variables|Default|GetStart%20Loc) (Variables|Default|GetEnd%20Loc) _alpha)))))
                    (:then_1
                      (Utilities|FlowControl|Delay 0.2)
                      (Audio|PlaySound2D "/Game/Audio/Sounds/phy_imp_cardox_wood_hvy_Cue.phy_imp_cardox_wood_hvy_Cue" 1.0 1.0 0.0 0 0))))))
            (:then_2
              (bind _progression_2 (Timeline|HoldItem_Opacity Play)
                (:Update
                  (Default|ProgressOpacity (Variables|/Game/Blueprints/myWorld/BP_Pawn.BP_Pawn_C|GetUI (Variables|Default|GetPawn)) _progression_2)))))
          (else
            (goto _label Reset)))))
    (else
      ;;;[0.1094 0.1094 0.1094] Detach from Pawn
      (Transformation|DetachFromComponent (Variables|Default|GetStaticMesh) "KeepWorld" "KeepWorld" "KeepWorld" true)
      (Rendering|SetRenderCustomDepth (Variables|Default|GetStaticMesh) true)
      ;;;[0.1094 0.1094 0.1094] Boolean Set
      (Variables|Default|SetIsPickedUp false)
      (Variables|/Game/Blueprints/myWorld/BP_Pawn.BP_Pawn_C|SetHeldItem (Variables|Default|GetPawn) 0)
      (Input|DisableInput (Game|GetPlayerController 0))
      (Default|EnableCrosshair (Variables|Default|GetPawn))
      (CallFunction|ResetMultiGate)
      (Timeline|PickupTimeline Reverse))))

(event Custom|Stop%20HoldClick
  (bind _pawn (Variables|Default|GetPawn))
  (bind _pawn_2 (Variables|Default|GetPawn))
  (bind _bpc_traceinteractor (Variables|/Game/Blueprints/myWorld/BP_Pawn.BP_Pawn_C|GetBPC_TraceInteractor _pawn))
  ;[1 1 1] Pick Up & Drop Item
  ;;[1 1 1] Hold Click Functionality
  ;;;[0.1094 0.1094 0.1094] Activate Input
  (Utilities|FlowControl|Sequence
    (:then_0
      (bind _progression (Timeline|HoldItem_Progress Stop)
        (:Update
          (Default|ProgressAlpha (Variables|/Game/Blueprints/myWorld/BP_Pawn.BP_Pawn_C|GetUI (Variables|Default|GetPawn)) _progression))
        (:Finished
          (CallFunction|StopHoldClick)
          ;;;[0.1094 0.1094 0.1094] Attach to Pawn
          (Rendering|SetRenderCustomDepth (Variables|Default|GetStaticMesh) false)
          (Variables|Default|SetEnd%20Loc (Math|Transform|MakeTransform (+ (Transformation|GetWorldLocation _bpc_traceinteractor) (* (Math|Vector|GetForwardVector _bpc_traceinteractor) 6e+01)) (.rotation (Variables|Default|GetStart%20Loc)) (.scale (Transformation|GetWorldTransform _bpc_traceinteractor))))
          (Transformation|SetMobility (Variables|Default|GetStaticMesh) "Movable")
          (Transformation|AttachComponentToComponent (Variables|/Game/Blueprints/myWorld/BP_Pawn.BP_Pawn_C|GetBPC_TraceInteractor (Variables|Default|GetPawn)) "None" "KeepWorld" "KeepWorld" "KeepWorld" true)
          ;;;[0.1094 0.1094 0.1094] Boolean Set
          (Variables|Default|SetIsPickedUp true)
          (Variables|/Game/Blueprints/myWorld/BP_Pawn.BP_Pawn_C|SetHeldItem (Variables|Default|GetPawn) self)
          (Default|DisableCrosshair (Variables|Default|GetPawn))
          (Utilities|FlowControl|Sequence
            (:then_0
              ;;;[0.1094 0.1094 0.1094] Transform Actor Location
              (bind _alpha (Timeline|PickupTimeline Play)
                (:Update
                  (if (> (.SphereRadius (Collision|GetComponentBounds (Variables|Default|GetStaticMesh))) 3e+01)
                    (Variables|Default|SetEnd%20Loc (Utilities|TraceTransform _pawn_2 8e+01))
                    (else
                      (Variables|Default|SetEnd%20Loc (Utilities|TraceTransform _pawn_2 4e+01))))
                  (Transformation|SetActorTransform (Math|Transform|Lerp(Transform) (Variables|Default|GetStart%20Loc) (Variables|Default|GetEnd%20Loc) _alpha)))))
            (:then_1
              (Utilities|FlowControl|Delay 0.2)
              (Audio|PlaySound2D "/Game/Audio/Sounds/phy_imp_cardox_wood_hvy_Cue.phy_imp_cardox_wood_hvy_Cue" 1.0 1.0 0.0 0 0))))))
    (:then_1
      (bind _progression_2 (Timeline|HoldItem_Opacity Reverse)
        (:Update
          (Default|ProgressOpacity (Variables|/Game/Blueprints/myWorld/BP_Pawn.BP_Pawn_C|GetUI (Variables|Default|GetPawn)) _progression_2))))))

(event EventBeginPlay
  ;[1 1 1] Beginplay - Set Variables
  (Variables|Default|SetStart%20Loc (Transformation|GetWorldTransform (Variables|Default|GetStaticMesh))) ; Save Start Location
  (Rendering|Material|SetScalarParameterValueonMaterials (Variables|Default|GetStaticMesh) "Opacity" 1.0)
  (bind _asbp_pawn (Utilities|Casting|CastToBP_Pawn (Game|Player|GetPlayerPawn 0))) ; Cast to Player Pawn
  (Variables|Default|SetPawn _asbp_pawn))

(event Input|AxisEvents|InputAxisLookUp
  (params (AxisValue :type Float%20%28single-precision%29))
  ;[1 1 1] RotateItem
  ;;[1 1 1] Rotate Item via input
  (Transformation|SetActorRotation (Math|Rotator|CombineRotators (Transformation|GetActorRotation) (Math|Rotator|MakeRotator (* AxisValue (Variables|/Game/Blueprints/myWorld/BP_Pawn.BP_Pawn_C|GetMouseSpeed (Variables|Default|GetPawn)) -1.0) 0.0 0.0))))

(event Input|AxisEvents|InputAxisTurn
  (params (AxisValue :type Float%20%28single-precision%29))
  ;[1 1 1] RotateItem
  ;;[1 1 1] Rotate Item via input
  (Transformation|SetActorRotation (Math|Rotator|CombineRotators (Transformation|GetActorRotation) (Math|Rotator|MakeRotator 0.0 0.0 (* AxisValue (Variables|/Game/Blueprints/myWorld/BP_Pawn.BP_Pawn_C|GetMouseSpeed (Variables|Default|GetPawn)) -1.0)))))

(fn ConstructionScript)

(fn TraceHitComponent
  (params (Hit :type Hit%20Result%20Structure) (Component :type Primitive%20Component%20Object%20Reference))
  (return false))

(fn TraceHitObject
  (params (Hit :type Hit%20Result%20Structure))
  (bind _staticmesh (Variables|Default|GetStaticMesh))
  (Rendering|SetCustomDepthStencilValue _staticmesh 253)
  (Rendering|SetRenderCustomDepth _staticmesh true)
  (return false))

(fn TraceLeaveComponent
  (params (Hit :type Hit%20Result%20Structure) (Component :type Primitive%20Component%20Object%20Reference))
  (return false))

(fn TraceLeaveObject
  (params (Hit :type Hit%20Result%20Structure))
  (bind _staticmesh (Variables|Default|GetStaticMesh))
  (Rendering|SetCustomDepthStencilValue _staticmesh 255)
  (Rendering|SetRenderCustomDepth _staticmesh false)
  (return false))

(fn TraceLeftPress
  (params (Hit :type Hit%20Result%20Structure) (Instigator :type Pawn%20Object%20Reference))
  (CallFunction|PickupItem) ; Fired from Pawn
  (return false))

(fn TraceLeftRelease
  (params (Hit :type Hit%20Result%20Structure) (Instigator :type Pawn%20Object%20Reference))
  (CallFunction|DropItem) ; Fired from Pawn
  (return false))

(fn TraceMove
  (params (Hit :type Hit%20Result%20Structure%20%28by%20ref%29))
  (return false))

(fn TraceRightPress
  (params (Hit :type Hit%20Result%20Structure) (Instigator :type Pawn%20Object%20Reference))
  (CallFunction|RotateItem) ; Fired from Pawn
  (return false))